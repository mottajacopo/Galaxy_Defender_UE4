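; Game mode Blueprint that tracks score, top score, enemy count and kills, and handles pausing.
; BeginPlay creates the HUD, showing it only in the Main level; PauseGame creates and reuses a pause menu.
; SaveScore writes high scores to an EndlessSaveGame, but its slot names are inconsistent and the load slot is empty.
; LoadScore is an empty stub, and UnPauseGame only unpauses, leaving the menu untouched.
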(event `self.ReceiveBeginPlay`
  (`WidgetBlueprintLibrary.SetInputMode_GameAndUIEx` (`GameplayStatics.GetPlayerController` 0) null "DoNotLock" false)
  (`self.SetScore` 0)
  (bind _returnvalue (`|CreateWidget` "/Game/Blueprints/UI/BP_W_HUD.BP_W_HUD_C"))
  (bind _output_get (set `self.BP W HUD` _returnvalue))
  (bind _returnvalue_2 (`GameplayStatics.GetCurrentLevelName` true))
  (if (`KismetStringLibrary.EqualEqual_StrStr` _returnvalue_2 "Main")
    (`UserWidget.AddToViewport` _output_get 0)))

(fn `EnemyKilled`
  (`/Engine/EditorBlueprintResources/StandardMacros.IncrementInt` (`self.EnemiesKilled`)
    (:`  `
      (`self.UpdateEnemyCount` -1))))

(fn `LoadScore`)

(fn `PauseGame`
  (`GameplayStatics.SetGamePaused` true)
  (`/Engine/EditorBlueprintResources/StandardMacros.IsValid` (`self.Pause Menu`)
    (:`Is Valid`
      _)
    (:`Is Not Valid`
      (bind _returnvalue (`|CreateWidget` "/Game/Blueprints/UI/PauseMenu.PauseMenu_C" (`GameplayStatics.GetPlayerController` 0)))
      (set `self.Pause Menu` _returnvalue)))
  (`UserWidget.AddToViewport` (`self.Pause Menu`) 0))

(fn `SaveScore`
  (bind _score (`self.Score`))
  (bind _returnvalue (`GameplayStatics.DoesSaveGameExist` "HighscoereData"))
  (if _returnvalue
    (bind _returnvalue_2 (`GameplayStatics.LoadGameFromSlot` ""))
    (bind _output_get (set `self.SaverSubClass` _returnvalue_2))
    (bind _asendless_save_game (cast `/Game/Blueprints/EndlessSaveGame` _output_get))
    (if (> _score (`/Game/Blueprints/EndlessSaveGame.HighScoreValue` _asendless_save_game))
      (set `/Game/Blueprints/EndlessSaveGame.HighScoreValue` _score _asendless_save_game)
      (`GameplayStatics.SaveGameToSlot` (`self.SaverSubClass`) "HighscoreData"))
    (else
      (bind _returnvalue_3 (`GameplayStatics.CreateSaveGameObject` "/Game/Blueprints/EndlessSaveGame.EndlessSaveGame_C"))
      (bind _output_get_2 (set `self.SaverSubClass` _returnvalue_3))
      (bind _asendless_save_game_2 (cast `/Game/Blueprints/EndlessSaveGame` _output_get_2))
      (set `/Game/Blueprints/EndlessSaveGame.HighScoreValue` _score _asendless_save_game_2)
      (`GameplayStatics.SaveGameToSlot` (`self.SaverSubClass`) "highscoreData"))))

(fn `SetScore`
  (params (A :type Integer))
  (bind _output_get (set `self.Score` (+ A (`self.Score`))))
  (if (>= _output_get (`self.TopScore`))
    (set `self.TopScore` (`self.Score`))
    (else
      (set `self.TopScore` (`self.TopScore`)))))

(fn `UnPauseGame`
  (`GameplayStatics.SetGamePaused` false))

(fn `UpdateEnemyCount`
  (params (Value :type Integer))
  (set `self.EnemyCount` (+ (`self.EnemyCount`) Value)))

(fn `UserConstructionScript`)
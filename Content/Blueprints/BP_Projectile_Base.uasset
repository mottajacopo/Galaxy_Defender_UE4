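; BP_Projectile_Base is a base projectile actor with a configurable glow colour, scale and speed.
; The Construction Script creates a dynamic glow material instance on the mesh, applies the scale, and sets the movement component's initial speed with no maximum speed cap.
; BeginPlay then pushes the projectile colour into that material.
; The graphs contain no overlap, hit or damage logic.
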(event `self.ReceiveBeginPlay`
  (`MaterialInstanceDynamic.SetVectorParameterValue` (`self.ProjectileMaterial`) "Colour" (`self.ProjectileColor`)))

(fn `UserConstructionScript`
  (bind _projectilemovement (`self.ProjectileMovement`))
  (bind _returnvalue (`PrimitiveComponent.CreateDynamicMaterialInstance` (`self.Projectile_Mesh`) 0 "/Game/Assets/Materials/Glow/M_Glow_Projectile_Inst.M_Glow_Projectile_Inst" "None"))
  (set `self.ProjectileMaterial` _returnvalue)
  (`SceneComponent.SetWorldScale3D` (`self.Projectile_Mesh`) (`self.Scale`))
  (set `ProjectileMovementComponent.InitialSpeed` (`self.Speed`) _projectilemovement)
  (set `ProjectileMovementComponent.MaxSpeed` 0.0 _projectilemovement))
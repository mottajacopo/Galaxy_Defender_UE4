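; Player Blueprint that plays a rising, spinning spawn animation, then moves on the X-Z plane from axis input.
; BeginPlay caches BP_GameMode and runs a timeline that lifts and rotates the actor, setting MovementEnabled when finished.
; UpDown and RightLeft axes set speeds that Tick applies as a swept per-frame offset, without delta-time scaling or checking MovementEnabled.
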(event `self.ReceiveBeginPlay`
  (bind _spawnlocation (`self.SpawnLocation`))
  (bind _asbp_game_mode (cast `/Game/Blueprints/BP_GameMode` (`GameplayStatics.GetGameMode`))
    (:`then`
      (set `self.BP_GameMode` _asbp_game_mode)
      (set `self.Yaw` (.yaw (`self.K2_GetActorRotation`)))
      (set `self.SpawnLocation` (`self.K2_GetActorLocation`))
      (bind (_direction _speed) (`Timeline|spawnAnimation`)
        (:`Update`
          (`self.K2_SetActorLocation` (`KismetMathLibrary.VLerp` _spawnlocation (+ _spawnlocation (0.0 0.0 100.0)) _speed))
          (`self.K2_SetActorRotation` (`KismetMathLibrary.RLerp` (`KismetMathLibrary.MakeRotator` 0.0 0.0 (+ (`self.Yaw`) 720.0)) (struct) _speed)))
        (:`Finished`
          (set `self.MovementEnabled` true))))
    (:`CastFailed`
      (`KismetSystemLibrary.PrintString` "BP not found"))))

(event `InputAxis|UpDown`
  (params (AxisValue :type "Float (single-precision)"))
  (set `self.VertSpeed` (* (`self.MovementSpeed`) AxisValue)))

(event `InputAxis|RightLeft`
  (params (AxisValue :type "Float (single-precision)"))
  (set `self.HorzSpeed` (* AxisValue (`self.MovementSpeed`))))

(event `self.ReceiveTick`
  (params (DeltaSeconds :type "Float (single-precision)"))
  (set `self.DeltaSeconds` DeltaSeconds)
  (`self.K2_SetActorLocation` (+ (`self.K2_GetActorLocation`) (`KismetMathLibrary.MakeVector` (`self.HorzSpeed`) 0.0 (`self.VertSpeed`))) true))

(fn `UserConstructionScript`)
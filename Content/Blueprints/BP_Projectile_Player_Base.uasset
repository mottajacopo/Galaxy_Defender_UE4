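; BP_Projectile_Player_Base is a base player projectile that damages whatever its mesh begins overlapping.
; The construction script creates a dynamic glow material, scales the mesh and sets the movement component's initial speed from variables, leaving max speed uncapped.
; BeginPlay tints that material with the projectile colour.
; On overlap it applies damage to the other actor, spawns a pixel explosion emitter and destroys itself.
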(event `self.ReceiveBeginPlay`
  (`MaterialInstanceDynamic.SetVectorParameterValue` (`self.ProjectileMaterial`) "Colour" (`self.ProjectileColor`)))

(event `self.Projectile_Mesh.OnComponentBeginOverlap`
  (params (OverlappedComponent :type "PrimitiveComponent Object Reference") (OtherActor :type "Actor Object Reference") (OtherComp :type "PrimitiveComponent Object Reference") (OtherBodyIndex :type Integer) (bFromSweep :type Boolean) (SweepResult :type "HitResult Structure (by ref)"))
  (`GameplayStatics.ApplyDamage` OtherActor (`self.Damage`))
  (`GameplayStatics.SpawnEmitterAtLocation` "/Game/Assets/Particles/P_Pixel_Explosion.P_Pixel_Explosion" (`self.K2_GetActorLocation`))
  (`self.K2_DestroyActor`))

(fn `UserConstructionScript`
  (bind _projectilemovement (`self.ProjectileMovement`))
  (bind _returnvalue (`PrimitiveComponent.CreateDynamicMaterialInstance` (`self.Projectile_Mesh`) 0 "/Game/Assets/Materials/Glow/M_Glow_Projectile_Inst.M_Glow_Projectile_Inst" "None"))
  (set `self.ProjectileMaterial` _returnvalue)
  (`SceneComponent.SetWorldScale3D` (`self.Projectile_Mesh`) (`self.Scale`))
  (set `ProjectileMovementComponent.InitialSpeed` (`self.Speed`) _projectilemovement)
  (set `ProjectileMovementComponent.MaxSpeed` 0.0 _projectilemovement))
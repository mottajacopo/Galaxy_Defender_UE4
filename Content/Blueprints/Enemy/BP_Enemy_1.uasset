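; BP_Enemy_1 is an enemy that moves along the world X axis and shoots at intervals when the player is near on that axis.
; Tick applies a swept move from speed and a direction flag while movement is enabled.
; The same Tick chain uses a short random Delay to pace fire, then checks X-only distance to the player pawn.
; Within range, it spawns a projectile at its own transform and plays a sound.
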(event `self.ReceiveBeginPlay`
  (`parent.ReceiveBeginPlay`))

(event `self.ReceiveTick`
  (params (DeltaSeconds :type "Float (single-precision)"))
  (bind _returnvalue (`GameplayStatics.GetPlayerPawn` 0))
  ;[1 1 1] Movement
  (if (`self.MoveEnabled`)
    (`self.K2_SetActorLocation` (+ (`self.K2_GetActorLocation`) (* (`KismetMathLibrary.MakeVector` (* (`self.Speed`) (`KismetMathLibrary.SelectFloat` 1.0 -1.0 (`self.MoveDirection`)))) DeltaSeconds)) true)
    ;[1 1 1] Fire Logic
    (`/Engine/EditorBlueprintResources/StandardMacros.IsValid` _returnvalue
      (:`Is Valid`
        (`KismetSystemLibrary.Delay` (`KismetMathLibrary.RandomFloatInRange` 0.1 0.4))
        (`/Engine/EditorBlueprintResources/StandardMacros.IsValid` (`GameplayStatics.GetPlayerPawn` 0)
          (:`Is Valid`
            (if (<= (`KismetMathLibrary.VSize` (* (- (`self.K2_GetActorLocation` _returnvalue) (`self.K2_GetActorLocation`)) (1.0 0.0 0.0))) (`self.DistanceFromPlayer`))
              (`|SpawnActorFromClass` (`self.ProjectileType`) (`self.GetTransform`) "AlwaysSpawn" "OverrideRootScale" null (struct) null)
              (`GameplayStatics.PlaySoundAtLocation` null (`self.K2_GetActorLocation`) (struct) 1.0 1.0 0.0 null null null))))))))

(fn `UserConstructionScript`
  (`parent.UserConstructionScript`))
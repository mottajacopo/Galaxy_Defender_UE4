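; Base enemy Blueprint that registers with BP_GameMode, randomizes direction and speed, and sets full health on spawn.
; A timeline lowers it 400 units into place, then enables movement, though no movement logic lives here.
; Non-projectile hits flip its direction, and player contact damages both sides.
; At zero health it spawns an explosion, reports the kill and score to the game mode, plays sound and destroys itself.
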(event `self.ReceiveBeginPlay`
  (bind _spawnlocation (`self.SpawnLocation`))
  ;[1 1 1] Setup reference and variables
  (bind _asbp_game_mode (cast `/Game/Blueprints/BP_GameMode` (`GameplayStatics.GetGameMode`)))
  (bind _output_get (set `self.BP_Gamemode` _asbp_game_mode))
  (`/Game/Blueprints/BP_GameMode.UpdateEnemyCount` _output_get 1)
  (set `self.MoveDirection` (`KismetMathLibrary.RandomBool`))
  (set `self.Speed` (`KismetMathLibrary.RandomFloatInRange` (`self.MinSpeed`) (`self.MaxSpeed`)))
  (set `self.SpawnLocation` (`self.K2_GetActorLocation`))
  (set `self.Health` (`self.MaxHealth`))
  ;[1 1 1] Spawn animation
  (bind (_direction _newtrack_0) (`Timeline|SpawnAnimation`)
    (:`Update`
      (`self.K2_SetActorLocation` (`KismetMathLibrary.VLerp` _spawnlocation (- _spawnlocation (0.0 0.0 400.0)) _newtrack_0)))
    (:`Finished`
      (set `self.MoveEnabled` true))))

(event `self.ReceiveHit`
  (params (MyComp :type "PrimitiveComponent Object Reference") (Other :type "Actor Object Reference") (OtherComp :type "PrimitiveComponent Object Reference") (bSelfMoved :type Boolean) (HitLocation :type "Vector Structure") (HitNormal :type "Vector Structure") (NormalImpulse :type "Vector Structure") (Hit :type "HitResult Structure (by ref)"))
  ;[1 1 1] enemies hit logic
  (cast `/Game/Blueprints/Player/BP_Projectile_Player_Base` Other
    (:`CastFailed`
      (set `self.MoveDirection` (not (`self.MoveDirection`)))
      (bind _asbp_player (cast `/Game/Blueprints/Player/BP_Player` Other))
      (`GameplayStatics.ApplyDamage` _asbp_player 20.0)
      (`GameplayStatics.ApplyDamage` self 20.0)
      (`GameplayStatics.PlaySound2D` "/Game/Assets/Audio/mixkit-falling-hit-757.mixkit-falling-hit-757" 1.0 1.0 0.0 null null :!label _label))))

(event `self.ReceiveAnyDamage`
  (params (Damage :type "Float (single-precision)") (DamageType :type "DamageType Object Reference") (InstigatedBy :type "Controller Object Reference") (DamageCauser :type "Actor Object Reference"))
  ;[1 1 1] enemies hit logic
  (set `self.Health` (`KismetMathLibrary.FClamp` (- (`self.Health`) Damage) 0.0 (`self.MaxHealth`)))
  (if (<= (`self.Health`) 0.0)
    (`self.EnemyKilled`)
    (goto _label)))

(fn `EnemyKilled`
  (bind _bp_gamemode (`self.BP_Gamemode`))
  (`GameplayStatics.SpawnEmitterAtLocation` "/Game/Assets/Particles/P_Pixel_Explosion_Enemy.P_Pixel_Explosion_Enemy" (`self.K2_GetActorLocation`))
  (`/Game/Blueprints/BP_GameMode.EnemyKilled` _bp_gamemode)
  (`/Game/Blueprints/BP_GameMode.SetScore` _bp_gamemode (`self.EnemyScoreValue`))
  (`GameplayStatics.PlaySoundAtLocation` null (`self.K2_GetActorLocation`) (struct) 1.0 1.0 0.0 null null null)
  (`self.K2_DestroyActor`))

(fn `UserConstructionScript`)
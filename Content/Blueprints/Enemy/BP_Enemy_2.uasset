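; BP_Enemy_2 is an enemy actor that chases BP_Player while continuously spinning around its local pitch axis.
; Each Tick looks up the player and, if valid, makes a swept constant-speed interpolated move toward its location, scaled by MinSpeed.
; The move pairs a fixed 60 fps interp timestep with a speed scaled by DeltaSeconds, and the spin is likewise delta-scaled, keeping both frame-rate independent.
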(event `self.ReceiveBeginPlay`
  (`parent.ReceiveBeginPlay`))

(event `self.ReceiveTick`
  (params (DeltaSeconds :type "Float (single-precision)"))
  ;[1 1 1] movement and rotation
  (set `self.Delta Seconds` DeltaSeconds)
  (bind _returnvalue (`GameplayStatics.GetActorOfClass` "/Game/Blueprints/Player/BP_Player.BP_Player_C"))
  (if (`KismetSystemLibrary.IsValid` _returnvalue)
    (`self.K2_SetActorLocation` (`KismetMathLibrary.VInterpTo_Constant` (`self.K2_GetActorLocation`) (`self.K2_GetActorLocation` _returnvalue) 0.0167 (* (/ (/ 60.0 0.3) (/ 1.0 (`self.Delta Seconds`))) (`self.MinSpeed`))) true)
    (`self.K2_AddActorLocalRotation` (`KismetMathLibrary.MakeRotator` 0.0 (/ (* 60.0 7.0) (/ 1.0 (`self.Delta Seconds`)))))))

(fn `UserConstructionScript`
  (`parent.UserConstructionScript`))
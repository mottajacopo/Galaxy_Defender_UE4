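; BP_Enemy_Asteroid is an enemy asteroid that drifts and tumbles across the X-Z plane.
; BeginPlay caches the game mode, randomizes speed limit and per-axis mesh scale, and launches it mostly along X or Z via ProjectileMovement.
; Tick rotates it and destroys it beyond fixed screen bounds.
; EnemyKilled passes its score to the game mode, plays explosion effects, destroys itself and has a one-in-three chance to spawn BP_Lives.
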(event `self.ReceiveBeginPlay`
  (bind _returnvalue (`KismetMathLibrary.RandomFloatInRange` -50.0 50.0))
  (bind _projectilemovement (`self.ProjectileMovement`))
  (bind _projectilemovement_2 (`self.ProjectileMovement`))
  (bind _returnvalue_2 (`KismetMathLibrary.RandomFloatInRange` (`self.MinScale`) (`self.MaxScale`)))
  (bind _returnvalue_3 (+ (`KismetMathLibrary.RandomFloatInRange` -1.0 1.0) 0.5))
  ;[1 1 1] Override begin play of enemy base
  (bind _asbp_game_mode (cast `/Game/Blueprints/GameMode/BP_GameMode` (`GameplayStatics.GetGameMode`)))
  (set `self.BP_Gamemode` _asbp_game_mode)
  (bind _output_get (set `self.Speed` (`KismetMathLibrary.RandomFloatInRange` (`self.MinSpeed`) (`self.MaxSpeed`))))
  (bind _output_get_2 (set `self.MaxSpeed` _output_get))
  (bind _output_get_3 (set `ProjectileMovementComponent.MaxSpeed` _output_get_2 _projectilemovement))
  (set `ProjectileMovementComponent.InitialSpeed` _output_get_3 _projectilemovement)
  (bind _output_get_4 (set `self.Scale` (`KismetMathLibrary.MakeVector` _returnvalue_2 _returnvalue_2 _returnvalue_2)))
  (`SceneComponent.SetWorldScale3D` (`self.StaticMesh`) _output_get_4)
  (if (`KismetMathLibrary.RandomBool`)
    (`ProjectileMovementComponent.SetVelocityInLocalSpace` _projectilemovement_2 (* (`KismetMathLibrary.MakeVector` 200.0 0.0 _returnvalue) _returnvalue_3))
    (else
      (`ProjectileMovementComponent.SetVelocityInLocalSpace` _projectilemovement_2 (* (`KismetMathLibrary.MakeVector` _returnvalue 0.0 200.0) _returnvalue_3)))))

(event `self.ReceiveTick`
  (params (DeltaSeconds :type "Float (single-precision)"))
  (bind (_returnvalue_x _returnvalue_y _returnvalue_z) (`KismetMathLibrary.BreakVector` (`self.K2_GetActorLocation`)))
  ;[1 1 1] Rotation
  (`self.K2_AddActorLocalRotation` (`KismetMathLibrary.MakeRotator` 0.2 (`KismetMathLibrary.RandomFloatInRange` 0.2 2.0) 0.2))
  ;[1 1 1] destroy asteorids when out of screen
  (if (or (> (`KismetMathLibrary.Abs` _returnvalue_x) 770.0) (> (`KismetMathLibrary.Abs` _returnvalue_z) 520.0))
    (`self.K2_DestroyActor`)))

(fn `EnemyKilled`
  (bind _returnvalue (`self.K2_GetActorLocation`))
  (`/Game/Blueprints/GameMode/BP_GameMode.SetScore` (`self.BP_Gamemode`) (`self.EnemyScoreValue`))
  (`GameplayStatics.PlaySoundAtLocation` null _returnvalue (struct) 1.0 1.0 0.0 null null null)
  (`GameplayStatics.SpawnEmitterAtLocation` "/Game/Assets/Particles/P_Pixel_Explosion.P_Pixel_Explosion" _returnvalue)
  (`self.K2_DestroyActor`)
  (if (== (`KismetMathLibrary.RandomIntegerInRange` 0 2) 0)
    (`|SpawnActorFromClass` "/Game/Blueprints/Player/BP_Lives.BP_Lives_C" (`KismetMathLibrary.Conv_VectorToTransform` _returnvalue) "Undefined" "OverrideRootScale" null null)))

(fn `UserConstructionScript`
  (`parent.UserConstructionScript`))
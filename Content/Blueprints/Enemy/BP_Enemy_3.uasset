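; BP_Enemy_3 is a laser enemy that moves vertically and damages BP_Player through its beam.
; While MoveEnabled, Tick sweeps it along Z at a per-frame random speed signed by MoveDirection, then calls LaserEmitter.
; LaserEmitter line-traces from StaticMesh to a rotated endpoint with debug drawing, stretches Laser to the hit distance and applies Damage every frame it hits the player.
; The Laser component-hit event is empty, leaving its damage nodes unconnected.
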(event `self.ReceiveTick`
  (params (DeltaSeconds :type "Float (single-precision)"))
  ;[1 1 1] Movement
  (if (`self.MoveEnabled`)
    (`self.K2_SetActorLocation` (+ (`self.K2_GetActorLocation`) (* (`KismetMathLibrary.MakeVector` 0.0 0.0 (* (`KismetMathLibrary.RandomFloatInRange` 100.0 300.0) (`KismetMathLibrary.SelectFloat` 1.0 -1.0 (`self.MoveDirection`)))) DeltaSeconds)) true)
    (`self.LaserEmitter`)))

(event `self.laser.OnComponentHit`
  (params (HitComponent :type "PrimitiveComponent Object Reference") (OtherActor :type "Actor Object Reference") (OtherComp :type "PrimitiveComponent Object Reference") (NormalImpulse :type "Vector Structure") (Hit :type "HitResult Structure (by ref)")))

(fn `LaserEmitter`
  (bind _staticmesh (`self.StaticMesh`))
  (bind _returnvalue (`SceneComponent.K2_GetComponentLocation` _staticmesh))
  (bind (_outhit _returnvalue_2) (`KismetSystemLibrary.LineTraceSingleByProfile` :`Start` _returnvalue :`End` (`KismetMathLibrary.GreaterGreater_VectorRotator` (+ _returnvalue (* (`SceneComponent.GetForwardVector` _staticmesh) 8888.0)) (struct :`Pitch` 94.0)) :`DrawDebugType` "ForOneFrame"))
  (if _returnvalue_2
    (bind (_bblockinghit _binitialoverlap _time _distance _location _impactpoint _normal _impactnormal _physmat _hitactor _hitcomponent _hitbonename _hititem _faceindex _tracestart) (`GameplayStatics.BreakHitResult` _outhit))
    (`SceneComponent.SetWorldScale3D` (`self.laser`) (`KismetMathLibrary.MakeVector` 0.1 0.1 (* (/ (`KismetMathLibrary.VSize` (- _location _tracestart)) 100.0) 2.0)))
    (bind _asbp_player (cast `/Game/Blueprints/Player/BP_Player` _hitactor))
    (`GameplayStatics.ApplyDamage` _asbp_player (`self.Damage`))))

(fn `UserConstructionScript`
  (`parent.UserConstructionScript`))
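; Game mode that tracks score, top score and enemy counts, and handles pausing.
; BeginPlay sets Game and UI input, runs the score save, and creates the HUD, showing it only in the "Main" level.
; SetScore adds to the running score, while SaveScore creates or updates the HighscoreValue save slot, overwriting only lower records.
; PauseGame pauses and shows a lazily created, reused pause menu.
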(event `self.ReceiveBeginPlay`
  (`WidgetBlueprintLibrary.SetInputMode_GameAndUIEx` (`GameplayStatics.GetPlayerController` 0) null "LockAlways" false)
  (`self.SetScore` 0)
  (`self.SaveScore`)
  (bind _returnvalue (`|CreateWidget` "/Game/Blueprints/UI/BP_HUD.BP_HUD_C"))
  (bind _output_get (set `self.BP W HUD` _returnvalue))
  (bind _returnvalue_2 (`GameplayStatics.GetCurrentLevelName` true))
  (if (`KismetStringLibrary.EqualEqual_StrStr` _returnvalue_2 "Main")
    (`UserWidget.AddToViewport` _output_get 0)))

(fn `EnemyKilled`
  (`/Engine/EditorBlueprintResources/StandardMacros.IncrementInt` (`self.EnemiesKilled`)
    (:`  `
      (`self.UpdateEnemyCount` -1))))

(fn `PauseGame`
  (`GameplayStatics.SetGamePaused` true)
  (`/Engine/EditorBlueprintResources/StandardMacros.IsValid` (`self.Pause Menu`)
    (:`Is Valid`
      _)
    (:`Is Not Valid`
      (bind _returnvalue (`|CreateWidget` "/Game/Blueprints/UI/BP_PauseMenu.BP_PauseMenu_C" (`GameplayStatics.GetPlayerController` 0)))
      (set `self.Pause Menu` _returnvalue)))
  (`UserWidget.AddToViewport` (`self.Pause Menu`) 0))

(fn `SaveScore`
  (bind _score (`self.Score`))
  (bind _returnvalue (`GameplayStatics.DoesSaveGameExist` "HighscoreValue"))
  (if _returnvalue
    (bind _returnvalue_2 (`GameplayStatics.LoadGameFromSlot` "HighscoreValue"))
    (bind _output_get (set `self.SaverSubClass` _returnvalue_2))
    (bind _asbp_save_game (cast `/Game/Blueprints/SaveGame/BP_SaveGame` _output_get))
    (if (> _score (`/Game/Blueprints/SaveGame/BP_SaveGame.HighScoreValue` _asbp_save_game))
      (set `/Game/Blueprints/SaveGame/BP_SaveGame.HighScoreValue` _score _asbp_save_game)
      (`GameplayStatics.SaveGameToSlot` (`self.SaverSubClass`) "HighscoreValue"))
    (else
      (bind _returnvalue_3 (`GameplayStatics.CreateSaveGameObject` "/Game/Blueprints/SaveGame/BP_SaveGame.BP_SaveGame_C"))
      (bind _output_get_2 (set `self.SaverSubClass` _returnvalue_3))
      (bind _asbp_save_game_2 (cast `/Game/Blueprints/SaveGame/BP_SaveGame` _output_get_2))
      (set `/Game/Blueprints/SaveGame/BP_SaveGame.HighScoreValue` _score _asbp_save_game_2)
      (`GameplayStatics.SaveGameToSlot` (`self.SaverSubClass`) "HighscoreValue"))))

(fn `SetScore`
  (params (A :type Integer))
  (bind _output_get (set `self.Score` (+ A (`self.Score`))))
  (if (>= _output_get (`self.TopScore`))
    (set `self.TopScore` (`self.Score`))
    (else
      (set `self.TopScore` (`self.TopScore`)))))

(fn `UnPauseGame`
  (`GameplayStatics.SetGamePaused` false))

(fn `UpdateEnemyCount`
  (params (Value :type Integer))
  (set `self.EnemyCount` (+ (`self.EnemyCount`) Value)))

(fn `UserConstructionScript`)
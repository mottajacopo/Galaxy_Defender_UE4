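; BP_Lives is a spinning pickup actor, apparently an extra life, though it changes no life count itself.
; BeginPlay scales up the Life component, and Tick rotates the actor on all three axes at a frame-rate-independent speed.
; Any overlap with Life destroys the actor before the BP_Player cast, so only the notification sound is limited to the player.
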(event `self.ReceiveBeginPlay`
  ;[1 1 1] set scale
  (`SceneComponent.SetWorldScale3D` (`self.Life`) (3.0 3.0 3.0)))

(event `self.ReceiveTick`
  (params (DeltaSeconds :type "Float (single-precision)"))
  ;[1 1 1] rotate
  (bind _output_get (set `self.deltaSeconds` DeltaSeconds))
  (bind _returnvalue (/ (* 60.0 0.6) (/ 1.0 _output_get)))
  (`self.K2_AddActorLocalRotation` (`KismetMathLibrary.MakeRotator` _returnvalue _returnvalue _returnvalue)))

(event `self.Life.OnComponentBeginOverlap`
  (params (OverlappedComponent :type "PrimitiveComponent Object Reference") (OtherActor :type "Actor Object Reference") (OtherComp :type "PrimitiveComponent Object Reference") (OtherBodyIndex :type Integer) (bFromSweep :type Boolean) (SweepResult :type "HitResult Structure (by ref)"))
  ;[1 1 1] destroy and play sound when overlapped
  (`self.K2_DestroyActor`)
  (cast `/Game/Blueprints/Player/BP_Player` OtherActor)
  (`GameplayStatics.PlaySound2D` "/Game/Assets/Audio/mixkit-sci-fi-positive-notification-266.mixkit-sci-fi-positive-notification-266" 2.0 1.0 0.0 null null))

(fn `UserConstructionScript`)
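; Player actor for an XZ-plane shooter, playing a rising spin on spawn and enabling movement only in the Main level.
; Tick applies interpolated axis input, aims the mesh via mouse ray-plane intersection, and updates weapon cooldowns.
; Timer-looped twin guns overheat, while the secondary fires a five-shot burst then recharges.
; Damage and BP_Lives pickups adjust health on BP_PlayerController, enemy hits bounce the player, and death opens GameOver and saves score.
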(event `self.ReceiveBeginPlay`
  (bind _spawnlocation (`self.SpawnLocation`))
  ;[1 1 1] SpawnAnimation
  (bind _asbp_game_mode (cast `/Game/Blueprints/GameMode/BP_GameMode` (`GameplayStatics.GetGameMode`))
    (:`then`
      (set `self.BP_GameMode` _asbp_game_mode)
      (set `self.Yaw` (.yaw (`self.K2_GetActorRotation`)))
      (set `self.SpawnLocation` (`self.K2_GetActorLocation`))
      (bind (_direction _speed) (`Timeline|spawnAnimation`)
        (:`Update`
          (`self.K2_SetActorLocation` (`KismetMathLibrary.VLerp` _spawnlocation (+ _spawnlocation (0.0 0.0 200.0)) _speed))
          (`SceneComponent.K2_SetRelativeRotation` (`self.Player_StaticMesh`) (`KismetMathLibrary.RLerp` (`KismetMathLibrary.MakeRotator` 0.0 0.0 (+ (`self.Yaw`) 720.0)) (struct) _speed) false false))
        (:`Finished`
          (bind _returnvalue (`GameplayStatics.GetCurrentLevelName` true))
          (if (`KismetStringLibrary.EqualEqual_StrStr` _returnvalue "Main")
            (set `self.MovementEnabled` true)))))
    (:`CastFailed`
      (`KismetSystemLibrary.PrintString` "BP not found"))))

(event `InputAxis|UpDown`
  (params (AxisValue :type "Float (single-precision)"))
  ;[1 1 1] Movement
  (bind _returnspeed (`self.Movement` AxisValue (`self.VertSpeed`)))
  (set `self.VertSpeed` _returnspeed))

(event `InputAxis|RightLeft`
  (params (AxisValue :type "Float (single-precision)"))
  ;[1 1 1] Movement
  (bind _returnspeed (`self.Movement` AxisValue (`self.HorzSpeed`)))
  (set `self.HorzSpeed` _returnspeed))

(event `self.ReceiveTick`
  (params (DeltaSeconds :type "Float (single-precision)"))
  (bind _returnvalue (`self.K2_GetActorLocation`))
  (bind _player_staticmesh (`self.Player_StaticMesh`))
  (bind (_worldlocation _worlddirection) (`PlayerController.DeprojectMousePositionToWorld` (`GameplayStatics.GetPlayerController` 0)))
  (bind (_t _intersection) (`KismetMathLibrary.LinePlaneIntersection_OriginNormal` _worldlocation (+ _worldlocation (* _worlddirection 5000.0)) _returnvalue (0.0 1.0 0.0)))
  (bind _pitch (.pitch (`KismetMathLibrary.FindLookAtRotation` _returnvalue _intersection)))
  ;[1 1 1] Movement
  (set `self.DeltaSeconds` DeltaSeconds)
  (`|ExecutionSequence`
    (:`then_0`
      (if (`self.MovementEnabled`)
        (`self.K2_SetActorLocation` (+ (`self.K2_GetActorLocation`) (`KismetMathLibrary.MakeVector` (`self.HorzSpeed`))) true)
        (`self.K2_SetActorLocation` (+ (`self.K2_GetActorLocation`) (`KismetMathLibrary.MakeVector` 0.0 0.0 (`self.VertSpeed`))) true)
        (`/Engine/EditorBlueprintResources/StandardMacros.IsValid` self
          (:`Is Valid`
            (`SceneComponent.K2_SetRelativeRotation` (`self.Player_StaticMesh`) (`KismetMathLibrary.RInterpTo_Constant` (`SceneComponent.GetSocketRotation` (`self.Player_StaticMesh`) "None") (`KismetMathLibrary.MakeRotator` 0.0 0.0 (+ (`self.Yaw`) (* (`self.HorzSpeed`) -7.0))) (`self.DeltaSeconds`) 150.0) false false)
            ;[1 1 1] Mouse rotate player
            (if (> (.pitch (`KismetMathLibrary.FindLookAtRotation` (`KismetMathLibrary.RotateAngleAxis` _returnvalue 90.0 (0.0 1.0 0.0)) (`KismetMathLibrary.RotateAngleAxis` _intersection 90.0 (0.0 1.0 0.0)))) 0.0)
              (`SceneComponent.K2_SetRelativeRotation` _player_staticmesh (`KismetMathLibrary.MakeRotator` 0.0 (* (+ _pitch 270.0) -1.0)) false false)
              (else
                (`SceneComponent.K2_SetRelativeRotation` _player_staticmesh (`KismetMathLibrary.MakeRotator` 0.0 (+ _pitch -90.0)) false false)))))))
    (:`then_1`
      (`self.PrimaryGunOverheat` false))
    (:`then_2`
      (`self.SecondaryGunRecharge` false))))

(event `Primary`
  ;[1 1 1] PrimaryFire
  (`self.PrimaryFire` (`SceneComponent.K2_GetComponentToWorld` (`self.ProjectileSpawnL`)) :!label _label)
  (`self.PrimaryFire` (`SceneComponent.K2_GetComponentToWorld` (`self.ProjectileSpawnR`)))
  (`self.PrimaryGunOverheat` true))

(event `InputAction|PrimaryWeapon`
  (params (Key :type "Key Structure"))
  ;[1 1 1] PrimaryFire
  (:`Pressed`
    (if (`self.MovementEnabled`)
      (if (not (`self.IsOverheated`))
        (`KismetSystemLibrary.K2_SetTimer` null "Primary" 0.2 true)
        (goto _label))))
  (:`Released`
    (`KismetSystemLibrary.K2_ClearTimer` null "Primary")))

(event `InputAction|Pause`
  (params (Key :type "Key Structure"))
  ;[1 1 1] Input Pause game
  (:`Pressed`
    (`/Game/Blueprints/GameMode/BP_GameMode.PauseGame` (`self.BP_GameMode`))))

(event `Secondary`
  (bind _returnvalue (`SceneComponent.K2_GetComponentToWorld` (`self.ProjectileSpawn`)))
  ;[1 1 1] SecondaryFire
  (`self.SecondaryFire` _returnvalue :!label _label_2)
  (`KismetSystemLibrary.Delay` 0.12)
  (`self.SecondaryFire` _returnvalue)
  (`KismetSystemLibrary.Delay` 0.12)
  (`self.SecondaryFire` _returnvalue)
  (`KismetSystemLibrary.Delay` 0.12)
  (`self.SecondaryFire` _returnvalue)
  (`KismetSystemLibrary.Delay` 0.12)
  (`self.SecondaryFire` _returnvalue)
  (`self.SecondaryGunRecharge` true))

(event `InputAction|SecondaryWeapon`
  (params (Key :type "Key Structure"))
  ;[1 1 1] SecondaryFire
  (:`Pressed`
    (if (`self.IsRecharging`)
      _
      (elif (`self.MovementEnabled`)
        (goto _label_2)))))

(event `self.ReceiveAnyDamage`
  (params (Damage :type "Float (single-precision)") (DamageType :type "DamageType Object Reference") (InstigatedBy :type "Controller Object Reference") (DamageCauser :type "Actor Object Reference"))
  ;[1 1 1] Damage logic
  (bind _asbp_player_controller (cast `/Game/Blueprints/Player/BP_PlayerController` (`GameplayStatics.GetPlayerController` 0)))
  (bind _output_get (set `self.BP_PlayerController` _asbp_player_controller))
  (bind _output (`/Game/Blueprints/Player/BP_PlayerController.SetHealth` _output_get (* -1 Damage)))
  (if (<= _output 0.0)
    (`GameplayStatics.SpawnEmitterAtLocation` "/Game/Assets/Particles/P_Pixel_Explosion.P_Pixel_Explosion" (`self.K2_GetActorLocation`))
    (`self.K2_DestroyActor`)
    ;[1 1 1] GameOver
    (`GameplayStatics.OpenLevel` "GameOver")
    ;[1 1 1] save score
    (`/Game/Blueprints/GameMode/BP_GameMode.SaveScore` (`self.BP_GameMode`))))

(event `self.Box Collider.OnComponentBeginOverlap`
  (params (OverlappedComponent :type "PrimitiveComponent Object Reference") (OtherActor :type "Actor Object Reference") (OtherComp :type "PrimitiveComponent Object Reference") (OtherBodyIndex :type Integer) (bFromSweep :type Boolean) (SweepResult :type "HitResult Structure (by ref)"))
  (bind _bp_playercontroller (`self.BP_PlayerController`))
  ;[1 1 1] Increase health when overlap BP_Lives
  (bind _asbp_lives (cast `/Game/Blueprints/Player/BP_Lives` OtherActor))
  (`/Engine/EditorBlueprintResources/StandardMacros.IsValid` _bp_playercontroller
    (:`Is Valid`
      (`/Game/Blueprints/Player/BP_PlayerController.SetHealth` _bp_playercontroller (`/Game/Blueprints/Player/BP_Lives.healthValue` _asbp_lives)))))

(event `self.Box Collider.OnComponentHit`
  (params (HitComponent :type "PrimitiveComponent Object Reference") (OtherActor :type "Actor Object Reference") (OtherComp :type "PrimitiveComponent Object Reference") (NormalImpulse :type "Vector Structure") (Hit :type "HitResult Structure (by ref)"))
  ;[1 1 1] Bounce if hit by enemy
  (cast `/Game/Blueprints/Enemy/BP_Enemy_Base` OtherActor)
  (set `self.HorzSpeed` (* 4.0 (.x Hit_Normal)))
  (set `self.VertSpeed` (* (.z Hit_Normal) 4.0))
  (`GameplayStatics.PlaySound2D` "/Game/Assets/Audio/mixkit-falling-hit-757.mixkit-falling-hit-757" 0.2 1.0 0.0 null null))

(fn `Movement`
  (params (Direction :type "Float (double-precision)") (CurrentSpeed :type "Float (double-precision)"))
  (returns (ReturnSpeed :type "Float (double-precision)"))
  (return (`KismetMathLibrary.FInterpTo` CurrentSpeed (* (`self.DeltaSeconds`) (* Direction (`self.MovementSpeed`))) (`self.DeltaSeconds`) 5.0)))

(fn `PrimaryFire`
  (params (Spawn :type "Transform Structure"))
  (locals (colour :type "LinearColor Structure" :default (struct :`G` 1.0 :`B` 0.035621)))
  (if (not (`self.IsOverheated`))
    (`|SpawnActorFromClass` "/Game/Blueprints/Player/BP_ProjectilePlayer_1.BP_ProjectilePlayer_1_C" Spawn "AlwaysSpawn" "OverrideRootScale" null (`local.colour`) self)
    (`GameplayStatics.PlaySoundAtLocation` "/Game/Assets/Audio/mixkit-short-laser-gun-shot-1670.mixkit-short-laser-gun-shot-1670" (`self.K2_GetActorLocation`) (struct) 1.0 1.0 0.0 null null null)))

(fn `PrimaryGunOverheat`
  (params (gunFired :type Boolean))
  (locals (increaseRate :type "Float (double-precision)" :default 0.14) (decreaseRate :type "Float (double-precision)" :default 0.006))
  (if gunFired
    ;[1 1 1] increase heat
    (bind _output_get (set `self.CurrentHeat` (+ (`self.CurrentHeat`) (`local.increaseRate`))))
    (set `self.IsOverheated` (>= (`KismetMathLibrary.FClamp` _output_get) 1.0))
    (else
      ;[1 1 1] decrease heat
      (if (> (`self.CurrentHeat`) 0.0)
        (set `self.CurrentHeat` (`KismetMathLibrary.FClamp` (- (`self.CurrentHeat`) (/ (* 60.0 (`local.decreaseRate`)) (/ 1.0 (`self.DeltaSeconds`))))))
        (if (== (`self.CurrentHeat`) 0.0)
          (set `self.IsOverheated` false))))))

(fn `SecondaryFire`
  (params (SpawnTrasnform :type "Transform Structure"))
  (locals (Colour :type "LinearColor Structure" :default (struct :`R` 0.973958 :`G` 0.319033)))
  (`|SpawnActorFromClass` "/Game/Blueprints/Player/BP_Projectile_Player_2.BP_Projectile_Player_2_C" SpawnTrasnform "AlwaysSpawn" "OverrideRootScale" null (`local.Colour`) self)
  (`GameplayStatics.PlaySoundAtLocation` "/Game/Assets/Audio/mixkit-laser-gun-shot-3110__1_.mixkit-laser-gun-shot-3110__1_" (`self.K2_GetActorLocation`) (struct) 0.7 1.0 0.0 null null null))

(fn `SecondaryGunRecharge`
  (params (gunFired :type Boolean))
  (locals (RechargeRate :type "Float (double-precision)" :default 0.003))
  (if gunFired
    ;[1 1 1] start timer
    (set `self.IsRecharging` true)
    (set `self.ChargeTime` 0.0)
    (else
      ;[1 1 1] recharging
      (if (`self.IsRecharging`)
        (set `self.ChargeTime` (`KismetMathLibrary.FClamp` (+ (`self.ChargeTime`) (/ (* 60.0 (`local.RechargeRate`)) (/ 1.0 (`self.DeltaSeconds`))))))
        (if (== (`self.ChargeTime`) 1.0)
          (set `self.IsRecharging` false))))))

(fn `UserConstructionScript`)